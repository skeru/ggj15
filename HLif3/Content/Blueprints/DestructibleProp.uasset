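; Destructible prop whose material and collision type reflect its current destruction level.
; Projectile overlaps call DestroyPartially with a negative step, while EditorCube11_Blueprint overlaps apply a positive step only if the prop is not yet destroyed.
; On each destruction-level update, the floored level selects the material, and the collision object type switches to Pawn when destroyed, otherwise PhysicsBody.
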(event EventOnDestroyLevelUpdate
  (Rendering|Material|SetMaterial 0 (Rendering|Material|GetMaterial (Math|Float|Floor (Variables|Default|GetDestructionLevel))))
  (bind _returnvalue (Class|DestructibleProp|IsDestroyed))
  (if _returnvalue
    (Collision|SetCollisionObjectType "ECC_Pawn")
    (else
      (Collision|SetCollisionObjectType "ECC_PhysicsBody"))))

(event EventActorBeginOverlap
  (params (OtherActor :type Actor%20Object%20Reference))
  (Utilities|Casting|CastToProjectile OtherActor
    (:then
      (Class|DestructibleProp|DestroyPartially -1.0))
    (:CastFailed
      (Utilities|Casting|CastToEditorCube11_Blueprint OtherActor)
      (bind _returnvalue (Class|DestructibleProp|IsDestroyed))
      (if (not _returnvalue)
        (Class|DestructibleProp|DestroyPartially 1.0)))))

(fn ConstructionScript)