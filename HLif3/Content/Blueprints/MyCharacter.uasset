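; MyCharacter is a character Blueprint that creates and owns the main UI widget.
; On BeginPlay it creates a UI_Main widget for its player controller, adds it to the viewport and keeps a reference.
; The G key feeds test messages to that widget and enables its news display, apparently as a debug trigger.
; A disconnected chain that would ask SteHLif3GameMode to spawn something at an index never runs.
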(event EventBeginPlay
  (bind _asplayer_controller (Utilities|Casting|CastToPlayerController (Pawn|GetController self)))
  (bind _returnvalue (UserInterface|CreateWidget "/Game/Blueprints/UI/UI_Main.UI_Main_C" _asplayer_controller))
  (UserInterface|Viewport|AddtoViewport _returnvalue)
  (Variables|Default|SetUIWidget _returnvalue))

(event Input|KeyboardEvents|G
  (bind _uiwidget (Variables|Default|GetUIWidget))
  (:Pressed
    (Default|SetMessageBundle _uiwidget (Utilities|Array|MakeArray "Test 1" "Test 2" "Test 3"))
    (Default|EnableNews _uiwidget)))

(fn ConstructionScript)