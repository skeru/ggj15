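; AI controller for enemies that feeds the player's pawn to a behavior tree as its target.
; On BeginPlay it sets up the MoveFollow blackboard, stores player pawn 0 in the TargetLocation key and runs the CharacterMove behavior tree.
; Tick rewrites that key every frame with the current player pawn, stored as an object reference despite the key's name.
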(event EventBeginPlay
  (bind _self self)
  (Class|AIController|UseBlackboard _self "/Game/Bht/MoveFollow.MoveFollow")
  (AI|Components|Blackboard|SetValueasObject (AI|GetBlackboard _self) (Variables|Default|GetTargetLocation) (Game|Player|GetPlayerPawn 0))
  (AI|RunBehaviorTree "/Game/Bht/CharacterMove.CharacterMove"))

(event EventTick
  (params (DeltaSeconds :type Float%20%28single-precision%29))
  (AI|Components|Blackboard|SetValueasObject (AI|GetBlackboard 0) (Variables|Default|GetTargetLocation) (Game|Player|GetPlayerPawn 0)))

(fn ConstructionScript)