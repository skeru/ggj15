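; Enemy projectile that raises corruption when it touches the player and can be shot down by player projectiles.
; On BeginPlay it loads its enemy descriptor from the default for its projectile type.
; Each hit from a PlayerProjectile rebuilds the descriptor with one less health, destroying the actor when none remains.
; Overlapping the player character notifies the first CorruptionManager found in the level, then destroys the projectile.
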(event EventActorBeginOverlap
  (params (OtherActor :type Actor%20Object%20Reference))
  (Utilities|Casting|CastToHLif3Character OtherActor)
  (bind _outactors (Actor|GetAllActorsOfClass "/Script/HLif3.CorruptionManager"))
  (bind _ascorruption_manager (Utilities|Casting|CastToCorruptionManager (Utilities|Array|Get(acopy) _outactors)))
  (Class|CorruptionManager|OnCorruptionIncrease _ascorruption_manager 1e+01)
  (Actor|DestroyActor))

(event EventBeginPlay
  (bind _returnvalue (Class|EnemyProjectile|GetDefaultDescriptor self (Variables|Default|GetPrType)))
  (Variables|Default|SetDescriptor _returnvalue))

(event EventHit
  (params (MyComp :type Primitive%20Component%20Object%20Reference) (Other :type Actor%20Object%20Reference) (OtherComp :type Primitive%20Component%20Object%20Reference) (bSelfMoved :type Boolean) (HitLocation :type Vector :default "0, 0, 0") (HitNormal :type Vector :default "0, 0, 0") (NormalImpulse :type Vector :default "0, 0, 0") (Hit :type Hit%20Result%20Structure%20%28by%20ref%29))
  (Utilities|Casting|CastToPlayerProjectile Other)
  (Math|Integer|CompareInt (- (.Health (Utilities|Struct|BreakEnemyDescriptor (Variables|Default|GetDescriptor))) 1) 0
    (:>
      (Variables|Default|SetDescriptor (Utilities|Struct|MakeEnemyDescriptor (- (.Health (Utilities|Struct|BreakEnemyDescriptor (Variables|Default|GetDescriptor))) 1) (.Speed (Utilities|Struct|BreakEnemyDescriptor (Variables|Default|GetDescriptor))) (.Movement (Utilities|Struct|BreakEnemyDescriptor (Variables|Default|GetDescriptor))) (.Target (Utilities|Struct|BreakEnemyDescriptor (Variables|Default|GetDescriptor))) (.Attak (Utilities|Struct|BreakEnemyDescriptor (Variables|Default|GetDescriptor))))))
    (:==
      (Actor|DestroyActor :!label _label))
    (:<
      (goto _label))))

(fn ConstructionScript)