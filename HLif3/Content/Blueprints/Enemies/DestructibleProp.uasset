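; Destructible prop that enemy projectiles damage and player projectiles repair, tied to the game's corruption level.
; Overlaps step the destruction level via DestroyPartially; enemy hits only count until the prop is destroyed.
; A player hit on a destroyed prop also lowers corruption through the CorruptionManager, found with GetAllActorsOfClass.
; Level updates swap the material by floored destruction level and toggle collision object type between Pawn (destroyed) and PhysicsBody.
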(event EventOnDestroyLevelUpdate
  (Rendering|Material|SetMaterial 0 (Rendering|Material|GetMaterial (Math|Float|Floor (Variables|Default|GetDestructionLevel))))
  (bind _returnvalue (Class|DestructibleProp|IsDestroyed))
  (if _returnvalue
    (Collision|SetCollisionObjectType "ECC_Pawn")
    (else
      (Collision|SetCollisionObjectType "ECC_PhysicsBody"))))

(event EventActorBeginOverlap
  (params (OtherActor :type Actor%20Object%20Reference))
  (Utilities|Casting|CastToPlayerProjectile OtherActor
    (:then
      (bind _returnvalue (Class|DestructibleProp|IsDestroyed))
      (if _returnvalue
        (bind _outactors (Actor|GetAllActorsOfClass "/Script/HLif3.CorruptionManager"))
        (bind _ascorruption_manager (Utilities|Casting|CastToCorruptionManager (Utilities|Array|Get(acopy) _outactors)))
        (Class|CorruptionManager|OnCorruptionIncrease _ascorruption_manager -1e+01))
      (Class|DestructibleProp|DestroyPartially -1.0))
    (:CastFailed
      (Utilities|Casting|CastToEnemyProjectile OtherActor)
      (bind _returnvalue_2 (Class|DestructibleProp|IsDestroyed))
      (if (not _returnvalue_2)
        (Class|DestructibleProp|DestroyPartially 1.0)))))

(fn ConstructionScript)