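; EditorCube11_Blueprint is a gravity-free physics enemy that chases the player through a constant force applied toward them every tick.
; Overlapping any Character raises corruption through the level's CorruptionManager, then calls DestroyComponent.
; Projectile hits add points to a ScoreBoard found at BeginPlay, without destroying the enemy.
; The construction script and NewFunction_0 are empty.
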(event EventTick
  (params (DeltaSeconds :type Float%20%28single-precision%29))
  (Physics|AddForce (* (Class|KismetMathLibrary|GetDirectionVector (Transformation|GetActorLocation) (Transformation|GetActorLocation (Game|GetPlayerCharacter 0))) 1e+05) "None"))

(event EventBeginPlay
  (Physics|SetEnableGravity false)
  (bind _outactors (Actor|GetAllActorsOfClass "/Game/Blueprints/ScoreBoard.ScoreBoard_C"))
  (Variables|Default|SetScoreBoard (Utilities|Array|Get(acopy) _outactors)))

(event EventActorBeginOverlap
  (params (OtherActor :type Actor%20Object%20Reference))
  (Utilities|Casting|CastToCharacter OtherActor)
  (bind _outactors (Actor|GetAllActorsOfClass "/Script/HLif3.CorruptionManager"))
  (bind _ascorruption_manager (Utilities|Casting|CastToCorruptionManager (Utilities|Array|Get(acopy) _outactors)))
  (Class|CorruptionManager|OnCorruptionIncrease _ascorruption_manager 1e+01)
  (Components|DestroyComponent))

(event EventHit
  (params (MyComp :type Primitive%20Component%20Object%20Reference) (Other :type Actor%20Object%20Reference) (OtherComp :type Primitive%20Component%20Object%20Reference) (bSelfMoved :type Boolean) (HitLocation :type Vector :default "0, 0, 0") (HitNormal :type Vector :default "0, 0, 0") (NormalImpulse :type Vector :default "0, 0, 0") (Hit :type Hit%20Result%20Structure%20%28by%20ref%29))
  (Utilities|Casting|CastToProjectile Other)
  (Class|ScoreBoard|AddPoints (Variables|Default|GetScoreBoard) 1e+02))

(fn ConstructionScript)

(fn NewFunction0)