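; Sound manager Blueprint that plays music tracks from its Music array, starting with the first on BeginPlay.
; NextSong and PreviousSong events step an index, clamp it between the first and third entries, then replay through the shared PlaySoundAttached call.
; Each call attaches a new sound to an audio component created at BeginPlay, with no stop of the previous track.
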(event EventNextSong
  (Variables|Default|SetIndex (+ (Variables|Default|GetIndex) 1))
  (if (>= (Variables|Default|GetIndex) 2)
    (Variables|Default|SetIndex 2))
  (Class|GameplayStatics|PlaySoundAttached (Utilities|Array|Get(acopy) (Variables|Default|GetMusic) (Variables|Default|GetIndex)) (stale EventBeginPlay _returnvalue)))

(event EventPreviousSong
  (Variables|Default|SetIndex (+ (Variables|Default|GetIndex) -1))
  (if (<= (Variables|Default|GetIndex) 0)
    (Variables|Default|SetIndex 0))
  (Class|GameplayStatics|PlaySoundAttached (Utilities|Array|Get(acopy) (Variables|Default|GetMusic) (Variables|Default|GetIndex)) (stale EventBeginPlay _returnvalue)))

(event EventBeginPlay
  (Variables|Default|SetIndex 0)
  (bind _returnvalue (AddComponent|AddAudioComponent false))
  (Class|GameplayStatics|PlaySoundAttached (Utilities|Array|Get(acopy) (Variables|Default|GetMusic) (Variables|Default|GetIndex)) _returnvalue))

(fn ConstructionScript)