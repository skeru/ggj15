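; Game mode that ties the screen's fringe post-process effect to the level of corruption.
; On BeginPlay it spawns a CorruptionManager at the origin and caches it along with the first PostProcessVolume found in the level.
; Each Tick it samples the FringeOverTime curve at current over maximum corruption and applies the result as that volume's fringe intensity.
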(event EventBeginPlay
  (Game|SpawnActorfromClass "/Game/Blueprints/GamePlay/CorruptionManager.CorruptionManager_C" (Math|Transform|MakeTransform "0, 0, 0") false 0)
  (bind _outactors (Actor|GetAllActorsOfClass "/Script/Engine.PostProcessVolume"))
  (Variables|Default|SetPostProcess (Utilities|Array|Get(acopy) _outactors))
  (bind _outactors_2 (Actor|GetAllActorsOfClass "/Game/Blueprints/GamePlay/CorruptionManager.CorruptionManager_C"))
  (Variables|Default|SetCorruptionManager (Utilities|Array|Get(acopy) _outactors_2)))

(event EventTick
  (params (DeltaSeconds :type Float%20%28single-precision%29))
  (bind _corruptionmanager (Variables|Default|GetCorruptionManager))
  (Class|HLif3GameMode|EditFringeIntensity (Variables|Default|GetPostProcess) (Math|Curves|GetFloatValue (Variables|Default|GetFringeOverTime) (/ (Variables|/Script/HLif3.CorruptionManager|GetCorruptionLevel _corruptionmanager) (Variables|/Script/HLif3.CorruptionManager|GetMaxCorruption _corruptionmanager)))))

(fn ConstructionScript)