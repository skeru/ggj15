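; Physics-driven pursuer actor that homes in on the player and raises corruption on contact.
; Each tick it applies a constant-magnitude force toward player character 0, with no delta-time scaling.
; Overlapping any Character reports a fixed increase to the level's CorruptionManager, then destroys the actor.
; BeginPlay caches the first ScoreBoard in the level, though these graphs never use it.
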(event EventTick
  (params (DeltaSeconds :type Float%20%28single-precision%29))
  (Physics|AddForce (* (Class|KismetMathLibrary|GetDirectionVector (Transformation|GetActorLocation) (Transformation|GetActorLocation (Game|GetPlayerCharacter 0))) 1e+05) "None"))

(event EventBeginPlay
  (bind _outactors (Actor|GetAllActorsOfClass "/Game/Blueprints/GamePlay/ScoreBoard.ScoreBoard_C"))
  (Variables|Default|SetScoreBoard (Utilities|Array|Get(acopy) _outactors)))

(event EventActorBeginOverlap
  (params (OtherActor :type Actor%20Object%20Reference))
  (Utilities|Casting|CastToCharacter OtherActor)
  (bind _outactors (Actor|GetAllActorsOfClass "/Script/HLif3.CorruptionManager"))
  (bind _ascorruption_manager (Utilities|Casting|CastToCorruptionManager (Utilities|Array|Get(acopy) _outactors)))
  (Class|CorruptionManager|OnCorruptionIncrease _ascorruption_manager 1e+01)
  (Actor|DestroyActor))

(fn ConstructionScript)