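; Corruption manager that partially destroys props in the level in response to corruption updates.
; On BeginPlay it caches every DestructibleProp and stores their count.
; Each corruption update prints the level and, if CanDestroy passes, calls DestroyPartially on the prop at the floored DestructibleIndex.
; CanDestroy and the index and level updates are defined outside this graph; game end only prints a debug message.
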(event EventBeginPlay
  (bind _destructibles (Variables|Default|GetDestructibles))
  (bind _outactors (Actor|GetAllActorsOfClass "/Game/Blueprints/DestructibleProp.DestructibleProp_C"))
  (for _array_element _outactors
    (bind _asdestructible_prop (Utilities|Casting|CastToDestructibleProp _array_element))
    (Utilities|Array|Add _destructibles _asdestructible_prop))
  (Variables|Default|SetDestructiblesLenght (Math|Conversions|ToFloat(Integer) (Utilities|Array|Length _destructibles))))

(event EventOnCorruptionUpdate
  (Development|PrintString (Utilities|String|Append "CORRUPTION: " (Utilities|String|ToString(Float) (Variables|Default|GetCorruptionLevel))) true true "(R=1.000000,G=0.458665,B=0.000000,A=1.000000)")
  (bind _returnvalue (Class|CorruptionManager|CanDestroy))
  (if _returnvalue
    (bind _asdestructible_prop (Utilities|Casting|CastToDestructibleProp (Utilities|Array|Get(acopy) (Variables|Default|GetDestructibles) (Math|Float|Floor (Variables|Default|GetDestructibleIndex)))))
    (Class|DestructibleProp|DestroyPartially _asdestructible_prop 1.0)))

(event EventOnGameEnd
  (Development|PrintString "GameOver" true true "(R=1.000000,G=0.027019,B=0.000000,A=1.000000)"))

(fn ConstructionScript)