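; Spawner actor that periodically spawns an AI pawn at its own location and rotation.
; Tick accumulates delta time in StartTime and resets it once the Duration threshold is reached.
; It then casts ToSpawn to Pawn and, on success, spawns it through SpawnAIFromClass with the CharacterMove behavior tree.
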(event EventTick
  (params (DeltaSeconds :type Float%20%28single-precision%29))
  (bind _self self)
  (Variables|Default|SetStartTime (+ DeltaSeconds (Variables|Default|GetStartTime)))
  (if (>= (+ DeltaSeconds (Variables|Default|GetStartTime)) (Variables|Default|GetDuration))
    (Variables|Default|SetStartTime 0.0)
    (bind _aspawn (Utilities|Casting|CastToPawnClass (Variables|Default|GetToSpawn)))
    (AI|SpawnAIFromClass _aspawn "/Game/Bht/CharacterMove.CharacterMove" (Transformation|GetActorLocation _self) (Transformation|GetActorRotation _self) false)))

(event EventBeginPlay)

(fn ConstructionScript)